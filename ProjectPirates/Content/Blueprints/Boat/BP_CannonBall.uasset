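; BP_CannonBall is a boat cannonball projectile that damages whatever it overlaps and destroys itself after 20 seconds.
; On sphere overlap it draws a debug sphere, then checks whether the other actor implements BPI_Damageable.
; Damageable actors receive a life decrease and a VFX message carrying the offset from the actor to the impact point, after which the ball is destroyed.
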(event OnComponentBeginOverlap(Sphere)
  (params (OverlappedComponent :type Primitive%20Component%20Object%20Reference) (OtherActor :type Actor%20Object%20Reference) (OtherComp :type Primitive%20Component%20Object%20Reference) (OtherBodyIndex :type Integer) (bFromSweep :type Boolean) (SweepResult :type Hit%20Result%20Structure%20%28by%20ref%29))
  (bind _staticmesh (Variables|Default|GetStaticMesh))
  (bind _returnvalue (Transformation|GetWorldLocation _staticmesh))
  (Rendering|Debug|DrawDebugSphere _returnvalue 1e+02 12 "(R=1.000000,G=1.000000,B=1.000000,A=1.000000)" 5.0)
  (if (Utilities|DoesObjectImplementInterface OtherActor "/Game/Blueprints/Interfaces/BPI_Damageable.BPI_Damageable_C")
    (Class|BPIDamageable|DecreaseLife(Message) OtherActor 1e+01)
    (Class|BPIDamageable|AddVFXs(Message) OtherActor (- _returnvalue (Transformation|GetActorLocation OtherActor)))
    (Actor|DestroyActor)))

(event Custom|Destroy%20Ball
  (Actor|DestroyActor)
  (Utilities|Time|ClearandInvalidateTimerbyHandle (stale EventBeginPlay _returnvalue)))

(event EventBeginPlay
  (bind _returnvalue (Utilities|Time|SetTimerbyEvent (delegate Custom|Destroy%20Ball) 2e+01)))

(event EventTick
  (params (DeltaSeconds :type Float%20%28single-precision%29)))

(fn ConstructionScript)