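; Damageable boat that exposes its static mesh as a buoyancy primitive and sinks when its health runs out.
; DecreaseLife subtracts damage and, at zero health, plays a timeline that rolls the mesh and raises its mass override to fake sinking.
; AddVFXs attaches an explosion, then a delayed fire, at the impact point, tracking both emitters so they are destroyed when the sinking timeline finishes.
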(event Custom|Remove%20VFXs
  (for _array_element (Variables|Default|GetArrayOfEffects)
    (Components|DestroyComponent _array_element)))

(event EventBeginPlay
  (Health|SetMaxCurrentHealth))

(event Collision|EventActorBeginOverlap
  (params (OtherActor :type Actor%20Object%20Reference)))

(event EventTick
  (params (DeltaSeconds :type Float%20%28single-precision%29)))

(event EventAddVFXs
  (params (PointOfImpact :type Vector :default "0, 0, 0"))
  (bind _staticmesh (Variables|Default|GetStaticMesh))
  (bind _returnvalue (Effects|SpawnEmitterAttached "/Game/StarterContent/Particles/P_Explosion.P_Explosion" _staticmesh "None" PointOfImpact "0, 0, 0" "1.000000,1.000000,1.000000" "KeepRelativeOffset" false))
  (Utilities|Array|Add (Variables|Default|GetArrayOfEffects) _returnvalue)
  (Utilities|FlowControl|Delay 0.2)
  (bind _returnvalue_2 (Effects|SpawnEmitterAttached "/Game/StarterContent/Particles/P_Fire.P_Fire" _staticmesh "None" PointOfImpact))
  (Utilities|Array|Add (Variables|Default|GetArrayOfEffects) _returnvalue_2))

(event EventDecreaseLife
  (params (DamageReceived :type Float%20%28double-precision%29))
  (bind _isdestroyed (Health|DecreaseHealth DamageReceived))
  (if _isdestroyed
    (Variables|Default|SetoldRot (Transformation|GetActorRotation self))
    (bind _newtrack_0 (Timeline|Timeline Play)
      (:Update
        (CallFunction|SinkingShips _newtrack_0))
      (:Finished
        (CallFunction|RemoveVFXs)))))

(fn ConstructionScript)

(fn GetBuoyancyPontoons
  (return 0))

(fn GetBuoyancyPrimitive
  (return (Variables|Default|GetStaticMesh)))

(fn SetMaxCurrentHealth
  (Variables|Health|SetCurrentHealth (Variables|Health|GetMaxHealth)))

(fn DecreaseHealth
  (params (Damage :type Float%20%28double-precision%29))
  (if (<= (- (Variables|Health|GetCurrentHealth) Damage) 0.0)
    (Variables|Health|SetCurrentHealth 0.0)
    (return true)
    (else
      (Variables|Health|SetCurrentHealth (- (Variables|Health|GetCurrentHealth) Damage))
      (return false))))

(fn SinkingShips
  (params (NewParam :type Float%20%28double-precision%29))
  (bind _oldrot (Variables|Default|GetoldRot))
  (bind _staticmesh (Variables|Default|GetStaticMesh))
  (Transformation|SetRelativeRotation _staticmesh (Math|Rotator|MakeRotator (Math|Float|Lerp 0.0 2e+01 NewParam) (.pitch _oldrot) (.yaw _oldrot)) false false)
  (Class|PrimitiveComponent|SetMassOverrideinKg _staticmesh "None" (Math|Float|Lerp 2e+02 8e+02 NewParam) true))